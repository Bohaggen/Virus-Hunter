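; Base gun Blueprint that handles firing, reloading, hit damage, impact effects and scope render-target capture.
; SwitchTrigger feeds ShootBullet, which checks character state and ammo, then fires once for Burst or re-arms a timer for Auto.
; Each shot traces from the muzzle along ScopeCamera, doubles head-bone damage, adds recoil, effects and physics force, and spawns a projectile at impact.
; Reloading plays paired montages, toggles bullet-bone visibility through notifies and refills the clip from reserve on completion.
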(event `reloading`
  (bind _character (`self.Character`))
  (bind _fp_gun (`self.FP_Gun`))
  ;[1 0.4369 0] Reloading
  (if (!= (`self.CurrentClip`) (`self.ClipSize`))
    (if (> (`self.Bullet`) 0)
      (set `self.IsReloading?` true)
      (bind _notifyname (`|PlayMontage` (`self.FP_Gun`) (`self.ReloadAnimMontage_Weapon`) 1.5 0.0 "Default")
        (:`then`
          (set `/Game/GAM_305/Blueprints/BP_FPSCharacter.IsReloading?` true _character)
          (`|PlayMontage` (`Character.Mesh` _character) (`self.reloadAnimMontage`) 1.5
            (:`OnCompleted`
              (set `/Game/GAM_305/Blueprints/BP_FPSCharacter.IsReloading?` false _character)
              (set `self.IsReloading?` false)
              (if (> (+ (`self.Bullet`) (`self.CurrentClip`)) (`self.ClipSize`))
                (set `self.Bullet` (+ (- (`self.CurrentClip`) (`self.ClipSize`)) (`self.Bullet`)))
                (set `self.CurrentClip` (`self.ClipSize`))
                (else
                  (set `self.CurrentClip` (+ (`self.Bullet`) (`self.CurrentClip`)))
                  (set `self.Bullet` 0))))))
        (:`OnNotifyBegin`
          (switch `name` _notifyname
            (:`unHide`
              (`SkinnedMeshComponent.UnHideBoneByName` _fp_gun "bullets"))
            (:`hide`
              (`SkinnedMeshComponent.HideBoneByName` _fp_gun "bullets" "PBO_None"))))))))

(event `DrawingScope`
  ;[1 0.4369 0] Scope
  (set `SceneCaptureComponent2D.TextureTarget` "/Game/GAM_305/Textures/RT_Scope.RT_Scope" (`self.Scope_Capture`)))

(event `self.ReceiveBeginPlay`
  ;[1 0.4369 0] Initialize
  (`self.initializeWeapon`))

(event `playShootingMontage`
  (bind _animweaponshootmontage (`self.AnimWeaponShootMontage`))
  ;[1 0.4369 0] Play Montage
  (`|PlayMontage` (`Character.Mesh` (`self.Character`)) (`self.animShootingMontage`)
    (:`then`
      (`/Engine/EditorBlueprintResources/StandardMacros.IsValid` _animweaponshootmontage
        (:`Is Valid`
          (`|PlayMontage` (`self.FP_Gun`) _animweaponshootmontage))))))

(event `StopDrawingScope`
  ;[1 0.4369 0] Scope
  (set `SceneCaptureComponent2D.TextureTarget` null (`self.Scope_Capture`)))

(event `InitializeWeapon`
  ;[1 0.4369 0] Initialize
  (set `self.FOV` (`CameraComponent.FieldOfView` (`self.ScopeCamera`)))
  (`KismetSystemLibrary.Delay` 10.0)
  (`PrimitiveComponent.SetSimulatePhysics` (`self.FP_Gun`) false))

(event `ImpactFX`
  (params (Emitter :type "ParticleSystem Object Reference") (AttachToComponent :type "SceneComponent Object Reference") (AttachPointName :type Name) (Location :type "Vector Structure") (DecalMaterial :type "MaterialInterface Object Reference") (Rotation :type "Rotator Structure") (Target :type "PrimitiveComponent Object Reference"))
  (bind _fp_gun (`self.FP_Gun`))
  ;[1 0.4369 0] Impact effects
  (`/Engine/EditorBlueprintResources/StandardMacros.IsValid` _fp_gun
    (:`Is Valid`
      (`GameplayStatics.SpawnEmitterAttached` "/Game/GAM_305/Effects/MuzzleFlash/P_Muzzle.P_Muzzle" _fp_gun "Muzzle" (`SceneComponent.GetSocketLocation` _fp_gun "Muzzle") (`SceneComponent.GetSocketRotation` _fp_gun "Muzzle") (1.0 1.0 1.0) "KeepWorldPosition")
      (`GameplayStatics.SpawnEmitterAttached` Emitter AttachToComponent AttachPointName Location Rotation (1.0 1.0 1.0) "KeepWorldPosition")
      (`GameplayStatics.SpawnDecalAttached` DecalMaterial (7.0 7.0 7.0) AttachToComponent AttachPointName Location Rotation "KeepWorldPosition" 120.0)
      (`GameplayStatics.PlaySoundAtLocation` (`self.ShootSound`) (`SceneComponent.K2_GetComponentLocation` (`self.FP_Gun`)) (struct) 1.0 1.0 0.0 null null null)
      (`/Engine/EditorBlueprintResources/StandardMacros.IsValid` Target
        (:`Is Valid`
          (`self.Physics` Target))))))

(event `Physics`
  (params (AttachToComponent :type "PrimitiveComponent Object Reference"))
  ;[1 0.4369 0] Impact effects
  (if (`SceneComponent.IsSimulatingPhysics` AttachToComponent "None")
    (`PrimitiveComponent.AddForce` AttachToComponent (* (`SceneComponent.GetForwardVector` (`self.cameraActive`)) 5000.0) "None" true)))

(event `SwitchTrigger`
  (params (isFiring :type Boolean) (Instigator :type "Controller Object Reference") (Camera :type "CameraComponent Object Reference") (character :type "/Game/GAM_305/Blueprints/BP_FPSCharacter Object Reference"))
  ;[1 0.4369 0] Shooting
  (set `self.Character` character)
  (set `self.Instigator ` Instigator)
  (set `self.cameraActive` Camera)
  (set `self.IsFiring?` isFiring)
  (`self.ShootBullet`))

(event `Shooting`
  (bind _character (`self.Character`))
  (bind _returnvalue (`SceneComponent.GetSocketLocation` (`self.FP_Gun`) "Muzzle"))
  ;[1 0.4369 0] Shooting
  (bind _outhit (`KismetSystemLibrary.LineTraceSingle` _returnvalue (+ _returnvalue (* (`SceneComponent.GetForwardVector` (`self.ScopeCamera`)) 1000000.0)) "TraceTypeQuery2"))
  (`/Engine/EditorBlueprintResources/StandardMacros.IsValid` _character
    (:`Is Valid`
      (set `/Game/GAM_305/Blueprints/BP_FPSCharacter.IsShooting?` true _character)
      (`self.SetDamage` _outhit)
      (`self.Recoil`)
      (bind (_bblockinghit _binitialoverlap _time _distance _location _impactpoint _normal) (`GameplayStatics.BreakHitResult` _outhit))
      (`|SpawnActorFromClass` "/Game/FirstPersonBP/Blueprints/FirstPersonProjectile1.FirstPersonProjectile1_C" (`KismetMathLibrary.MakeTransform` _location (`KismetMathLibrary.Conv_VectorToRotator` _normal)) "Undefined" "OverrideRootScale" null null))))

(event `SetDamage`
  (params (HitResult :type "HitResult Structure"))
  (bind (_bblockinghit _binitialoverlap _time _distance _location _impactpoint _normal _impactnormal _physmat _hitactor _hitcomponent _hitbonename) (`GameplayStatics.BreakHitResult` HitResult))
  ;[1 0.4369 0] Shooting
  (bind _damage (`self.Damage` _hitbonename))
  (if (!= (`self.Character`) _hitactor)
    (`GameplayStatics.ApplyPointDamage` _hitactor _damage _location HitResult (`self.Instigator `) (`self.Character`)))
  (`self.ImpactFX` "/Game/GAM_305/Effects/MuzzleFlash/P_hit_effect.P_hit_effect" _hitcomponent _hitbonename _location "/Game/GAM_305/Materials/MI_Bullet_Decals_Inst.MI_Bullet_Decals_Inst" (`KismetMathLibrary.Conv_VectorToRotator` _normal) _hitcomponent))

(event `Recoil`
  (bind _character (`self.Character`))
  ;[1 0.4369 0] Shooting
  (`/Engine/EditorBlueprintResources/StandardMacros.IsValid` _character
    (:`Is Valid`
      (`Pawn.AddControllerYawInput` _character (`KismetMathLibrary.RandomFloatInRange` -0.3 0.3))
      (`Pawn.AddControllerPitchInput` _character (`KismetMathLibrary.RandomFloatInRange` 0.1 -0.2))
      (if (`Pawn.IsLocallyControlled` _character)
        (`PlayerController.ClientStartCameraShake` :`self` (`GameplayStatics.GetPlayerController` 0) :`Shake` "/Game/GAM_305/Blueprints/BP_CameraShake.BP_CameraShake_C")))))

(fn `Damage`
  (params (bone :type Name))
  (returns (Damage :type "Float (double-precision)"))
  (locals (damageLocal :type "Float (double-precision)" :default 0.0))
  (bind _damagemin (`self.DamageMin`))
  (if (== bone "Head")
    (set `local.damageLocal` (* _damagemin 2.0))
    (else
      (set `local.damageLocal` _damagemin)))
  (return (`local.damageLocal`)))

(fn `ShootBullet`
  (bind _character (`self.Character`))
  (bind _character_2 (`self.Character`))
  (bind _currentclip (`self.CurrentClip`))
  (`/Engine/EditorBlueprintResources/StandardMacros.IsValid` _character
    (:`Is Valid`
      (if (`/Game/GAM_305/Blueprints/BP_FPSCharacter.IsHolstering?` _character)
        (set `self.IsFiring?` false :!label _label)
        (elif (`/Game/GAM_305/Blueprints/BP_FPSCharacter.IsReloading?` _character)
          (goto _label)
          (else
            _)))
      (if (`self.IsFiring?`)
        (if (> _currentclip 0)
          (set `self.CurrentClip` (- _currentclip 1))
          (switch `/Game/GAM_305/Blueprints/WeaponEnum/FireModeEnum` (`self.Firemode`)
            (:`NewEnumerator0`
              (`self.Shooting`))
            (:`NewEnumerator2`
              (`self.Shooting`)
              (`KismetSystemLibrary.K2_SetTimer` null "ShootBullet" (`self.FireSpeed`))))
          (`self.playShootingMontage`)
          (else
            (set `self.IsFiring?` false)
            (`/Engine/EditorBlueprintResources/StandardMacros.IsValid` _character_2 :!label _label_2
              (:`Is Valid`
                (set `/Game/GAM_305/Blueprints/BP_FPSCharacter.IsShooting?` false _character_2)))))
        (else
          (goto _label_2))))))

(fn `UserConstructionScript`)