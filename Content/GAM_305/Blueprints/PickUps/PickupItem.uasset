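; Pickup actor that grants the first-person player health, shield or ammo when walked over, based on its ItemType.
; BeginPlay applies the configured ItemMesh, and overlap casts to BP_FPSCharacter, then branches on the type to edit its stats directly.
; Health and active-weapon ammo are added without a cap, while full and partial shield refills check current Shield first.
; The pickup destroys itself only when its effect is applied.
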(event `self.ReceiveBeginPlay`
  (`StaticMeshComponent.SetStaticMesh` (`self.Default_Item`) (`self.Item_Mesh`)))

(event `self.ReceiveActorBeginOverlap`
  (params (OtherActor :type "Actor Object Reference"))
  (bind _asbp_fpscharacter (cast `/Game/GAM_305/Blueprints/BP_FPSCharacter` OtherActor))
  (if (`|EnumEquality` (`self.itemType`) "NewEnumerator0")
    (set `/Game/GAM_305/Blueprints/BP_FPSCharacter.Health` (+ (`/Game/GAM_305/Blueprints/BP_FPSCharacter.Health` _asbp_fpscharacter) 0.25) _asbp_fpscharacter)
    (`self.K2_DestroyActor`)
    (elif (`|EnumEquality` (`self.itemType`) "NewEnumerator1")
      (if (<= (`/Game/GAM_305/Blueprints/BP_FPSCharacter.Shield` _asbp_fpscharacter) 1.0)
        (set `/Game/GAM_305/Blueprints/BP_FPSCharacter.Shield` (`/Game/GAM_305/Blueprints/BP_FPSCharacter.MaxShield` _asbp_fpscharacter) _asbp_fpscharacter)
        (`self.K2_DestroyActor`))
      (elif (`|EnumEquality` (`self.itemType`) "NewEnumerator2")
        (bind _shield (`/Game/GAM_305/Blueprints/BP_FPSCharacter.Shield` _asbp_fpscharacter))
        (if (<= _shield 0.8)
          (set `/Game/GAM_305/Blueprints/BP_FPSCharacter.Shield` (+ _shield 0.2) _asbp_fpscharacter)
          (`self.K2_DestroyActor`))
        (elif (`|EnumEquality` (`self.itemType`) "NewEnumerator4")
          (bind _activeweapon (`/Game/GAM_305/Blueprints/BP_FPSCharacter.ActiveWeapon` _asbp_fpscharacter))
          (set `/Game/GAM_305/Blueprints/WeaponMaster.Bullet` (+ (`/Game/GAM_305/Blueprints/WeaponMaster.Bullet` _activeweapon) 15) _activeweapon)
          (`self.K2_DestroyActor`))))))

(fn `UserConstructionScript`)