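; Teleporter Blueprint that moves Characters entering its Portal to a linked Destination teleporter.
; The destination shifts the actor by the offset between the two teleporters and, unless KeepRotation is set, aligns actor and controller rotation to itself.
; An IncomingActors list blocks re-teleporting arrivals until they leave the Portal.
; The construction script tints a dynamic portal material with Color, or grey when no Destination is valid.
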(event `self.Portal.OnComponentBeginOverlap`
  (params (OverlappedComponent :type "PrimitiveComponent Object Reference") (OtherActor :type "Actor Object Reference") (OtherComp :type "PrimitiveComponent Object Reference") (OtherBodyIndex :type Integer) (bFromSweep :type Boolean) (SweepResult :type "HitResult Structure (by ref)"))
  (if (`self.CanTeleport?` OtherActor)
    (bind _destination (`self.Destination`)
      (:`then`
        (`self.IncomingTeleport` _destination OtherActor self))
      (:`else`))))

(event `self.Portal.OnComponentEndOverlap`
  (params (OverlappedComponent :type "PrimitiveComponent Object Reference") (OtherActor :type "Actor Object Reference") (OtherComp :type "PrimitiveComponent Object Reference") (OtherBodyIndex :type Integer))
  (`KismetArrayLibrary.Array_RemoveItem` (`self.IncomingActors`) OtherActor))

(event `IncomingTeleport`
  (params (IncomingActor :type "Actor Object Reference") (`Invoked Teleporter` :type "/Game/Additionals/Teleporter/Teleporter_BP Object Reference"))
  (`self.HandleTeleport` IncomingActor `Invoked Teleporter`))

(fn `CanTeleport?`
  (params (Actor :type "Actor Object Reference"))
  (returns (`CanTeleport?` :type Boolean))
  (cast `Character` Actor
    (:`then`
      (return (not (`KismetArrayLibrary.Array_Contains` (`self.IncomingActors`) (`local.Actor`)))))
    (:`CastFailed`
      (return false))))

(fn `HandleTeleport`
  (params (IncomingActor :type "Actor Object Reference") (`Invoked Teleporter` :type "/Game/Additionals/Teleporter/Teleporter_BP Object Reference"))
  (bind _returnvalue (`self.K2_GetActorRotation`))
  (bind _returnvalue_2 (`self.GetInstigatorController` (`local.IncomingActor`)))
  (if (not (`KismetArrayLibrary.Array_Contains` (`self.IncomingActors`) IncomingActor))
    (`KismetArrayLibrary.Array_Add` (`self.IncomingActors`) (`local.IncomingActor`))
    (`self.K2_SetActorLocation` (`local.IncomingActor`) (+ (`self.K2_GetActorLocation` (`local.IncomingActor`)) (- (`self.K2_GetActorLocation`) (`self.K2_GetActorLocation` (`local.Invoked Teleporter`)))) false true)
    (if (not (`self.KeepRotation`))
      (`self.K2_SetActorRotation` (`local.IncomingActor`) _returnvalue false)
      (`/Engine/EditorBlueprintResources/StandardMacros.IsValid` _returnvalue_2
        (:`Is Valid`
          (`Controller.SetControlRotation` _returnvalue_2 _returnvalue))))))

(fn `UserConstructionScript`
  (locals (MaterialInstance :type "MaterialInstanceDynamic Object Reference"))
  (bind _returnvalue (`KismetMaterialLibrary.CreateDynamicMaterialInstance` "/Game/Additionals/Teleporter/Teleporter_M.Teleporter_M"))
  (bind _output_get (set `local.MaterialInstance` _returnvalue))
  (`PrimitiveComponent.SetMaterial` (`self.Portal`) 0 _output_get)
  (`MaterialInstanceDynamic.SetVectorParameterValue` (`local.MaterialInstance`) "Color" (select `bool` (`KismetSystemLibrary.IsValid` (`self.Destination`)) :`false` (struct :`R` 0.416667 :`G` 0.416667 :`B` 0.416667 :`A` 1.0) :`true` (`self.Color`))))